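; BP_GAPAthComponent is an AI character path component that adds debug drawing of its path.
; On Tick, when Debug is on and the state is Active, it draws green lines over the 2D Steps points at the owner pawn's height, plus one from the pawn to the first step.
; The segment loop subtracts zero from the index, so each line starts and ends on the same point instead of joining consecutive steps.
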(event EventTick
  (params (DeltaSeconds :type Float%20%28single-precision%29))
  (if (Variables|Default|GetDebug)
    (if (Utilities|Enum|Equal(Enum) (Variables|Default|GetState) "GAPS_Active")
      (Variables|Default|SetZVal (.Z (Math|Vector|BreakVector (Transformation|GetActorLocation (Class|GAPathComponent|GetOwnerPawn)))))
      (for (_ _array_index) (Variables|Default|GetSteps)
        (if (> _array_index 0)
          (Rendering|Debug|DrawDebugLine (Math|Conversions|ToVector(Vector2D) (.Point (Utilities|Struct|BreakPathStep (Utilities|Array|Get(acopy) (Variables|Default|GetSteps) _array_index))) (Variables|Default|GetZVal)) (Math|Conversions|ToVector(Vector2D) (.Point (Utilities|Struct|BreakPathStep (Utilities|Array|Get(acopy) (Variables|Default|GetSteps) (- _array_index 0)))) (Variables|Default|GetZVal)) "(R=0.000000,G=1.000000,B=0.097295,A=1.000000)" 0.0 0.0)))
      (if (Utilities|Array|IsValidIndex (Variables|Default|GetSteps))
        (Rendering|Debug|DrawDebugLine (Math|Conversions|ToVector(Vector2D) (.Point (Utilities|Struct|BreakPathStep (Utilities|Array|Get(acopy) (Variables|Default|GetSteps)))) (Variables|Default|GetZVal)) (Transformation|GetActorLocation (Class|GAPathComponent|GetOwnerPawn)) "(R=0.000000,G=1.000000,B=0.097295,A=1.000000)" 0.0 0.0)))))