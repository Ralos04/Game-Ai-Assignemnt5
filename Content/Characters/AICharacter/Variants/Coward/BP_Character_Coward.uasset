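; Coward variant of the AI character that can shoot projectiles, self-destruct and break apart when killed.
; Shooting spawns the given projectile class at a shoot point, while self-destruct spawns a dedicated projectile at the actor before killing it through the vitality component.
; On death the capsule simulates physics until a looping timer finds it toppled, then the mesh parts detach as physics debris, capsule collision turns off and the controller unpossesses.
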(event Death(VitalityComponent_0)
  (Physics|SetSimulatePhysics (Variables|Default|GetCapsuleComponent) true)
  (bind _returnvalue (Utilities|Time|SetTimerbyEvent (delegate Custom|ToppleTimerCB) 0.3 true))
  (Variables|Default|SetToppleTimer_0 _returnvalue))

(event Custom|Shoot
  (params (ProjectileClass :type Actor%20Class%20Reference))
  (Game|SpawnActorfromClass ProjectileClass (Transformation|GetWorldTransform (Variables|Default|GetShootPoint_0)) "Undefined" "MultiplyWithRoot" 0 0))

(event Custom|ManualDeath
  (Default|Kill (Variables|Default|GetVitalityComponent_0)))

(event Custom|SelfDestruct
  (if (not (Variables|/Game/Characters/AICharacter/Variants/BP_VitalityComponent.BP_VitalityComponent_C|GetIsDead (Variables|Default|GetVitalityComponent_0)))
    (Game|SpawnActorfromClass "/Game/Characters/Projectiles/BP_SelfDestructProjectile.BP_SelfDestructProjectile_C" (Transformation|GetActorTransform) "Undefined" "MultiplyWithRoot" 0 0)
    (CallFunction|ManualDeath)))

(event Custom|ToppleTimerCB
  (bind _returnvalue (Pawn|GetController))
  (if (< (.Z (Math|Vector|BreakVector (Math|Vector|GetUpVector (Variables|Default|GetCapsuleComponent)))) 0.3)
    (Utilities|Time|ClearandInvalidateTimerbyHandle (Variables|Default|GetToppleTimer_0))
    (CallFunction|DetachandSimulate (Variables|Default|GetSphere))
    (CallFunction|DetachandSimulate (Variables|Default|GetSide2))
    (CallFunction|DetachandSimulate (Variables|Default|GetSide1))
    (CallFunction|DetachandSimulate (Variables|Default|GetFace1))
    (CallFunction|DetachandSimulate (Variables|Default|GetFace2))
    (CallFunction|DetachandSimulate (Variables|Default|GetCylinder))
    (CallFunction|DetachandSimulate (Variables|Default|GetTop))
    (CallFunction|DetachandSimulate (Variables|Default|GetBottom))
    (Physics|SetSimulatePhysics (Variables|Default|GetCapsuleComponent) false)
    (Collision|SetCollisionEnabled (Variables|Default|GetCapsuleComponent) "NoCollision")
    (Utilities|IsValid _returnvalue
      (:Is%20Valid
        (Pawn|UnPossess _returnvalue)))))

(fn ConstructionScript
  (|CallParentFunction))